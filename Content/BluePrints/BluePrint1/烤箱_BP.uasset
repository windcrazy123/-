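; Interactable oven Blueprint that bakes raw green or white mooncakes into their cooked versions.
; Overlapping its box as the TopDownCharacter shows a text prompt, enables input and opens a gate for the E key.
; E takes the raw mooncake from the HUD's left image slot, activates audio and shows a done text after a delay.
; State booleans track baking and type, and slot texture names serve as item IDs for loading and collecting.
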(event `Key|E`
  (params (Key :type "Key Structure"))
  (bind _textrender (`self.TextRender`))
  (bind _image_left (`/Game/UI/MyHUD.Image_left` (`/Game/TopDownBP/Blueprints/TopDownCharacter.hud` (`self.As Top Down Character`))))
  (bind _returnvalue (`KismetSystemLibrary.GetObjectName` (`WidgetBlueprintLibrary.GetBrushResourceAsTexture2D` (`Image.Brush` _image_left))))
  (bind _returnvalue_2 (== _returnvalue "青月饼（生）"))
  (:`Pressed`
    (`/Engine/EditorBlueprintResources/StandardMacros.Gate` true :!label _label
      (:`Exit`
        (if (`self.is doing`)
          _
          (elif (`self.is none`)
            (if (`KismetStringLibrary.EqualEqual_StrStr` _returnvalue "-1")
              (if (`self.is finished`) :!label _label_2
                (if (`self.is white`)
                  (`Image.SetBrushFromTexture` _image_left "/Game/UI/素材2/白月饼（熟）.白月饼（熟）" false)
                  (else
                    (`Image.SetBrushFromTexture` _image_left "/Game/UI/素材2/青月饼（熟）.青月饼（熟）" false)))
                (set `self.is finished` false)
                (set `self.is none` true)
                (`SceneComponent.SetVisibility` _textrender false false))
              (elif (or _returnvalue_2 (== _returnvalue "白月饼（生）"))
                (if _returnvalue_2
                  (set `self.is white` false)
                  (else
                    (set `self.is white` true)))
                (`Image.SetBrushFromTexture` _image_left "/Game/UI/素材/-1.-1" false)
                (set `self.is doing` true)
                (set `self.is none` false)
                (`ActorComponent.Activate` (`self.Audio`) false)
                (`KismetSystemLibrary.Delay` 8.0)
                (`SceneComponent.SetVisibility` _textrender true false)
                (set `self.is finished` true)
                (set `self.is doing` false)))
            (elif (`KismetStringLibrary.EqualEqual_StrStr` _returnvalue "-1")
              (goto _label_2))))))))

(event `self.Box.OnComponentBeginOverlap`
  (params (OverlappedComponent :type "PrimitiveComponent Object Reference") (OtherActor :type "Actor Object Reference") (OtherComp :type "PrimitiveComponent Object Reference") (OtherBodyIndex :type Integer) (bFromSweep :type Boolean) (SweepResult :type "HitResult Structure (by ref)"))
  (bind _astop_down_character (cast `/Game/TopDownBP/Blueprints/TopDownCharacter` OtherActor))
  (set `self.As Top Down Character` _astop_down_character)
  (`SceneComponent.SetVisibility` (`self.TextRender1`) true false)
  (`self.EnableInput` (`GameplayStatics.GetPlayerController` 0))
  (goto _label :!via `Open`))

(event `self.Box.OnComponentEndOverlap`
  (params (OverlappedComponent :type "PrimitiveComponent Object Reference") (OtherActor :type "Actor Object Reference") (OtherComp :type "PrimitiveComponent Object Reference") (OtherBodyIndex :type Integer))
  (cast `/Game/TopDownBP/Blueprints/TopDownCharacter` OtherActor)
  (`SceneComponent.SetVisibility` (`self.TextRender1`) false false)
  (`self.DisableInput` (`GameplayStatics.GetPlayerController` 0))
  (goto _label :!via `Close`))

(fn `UserConstructionScript`)
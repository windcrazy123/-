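; Trash can interactable that lets the player set HUD images while standing near it.
; A sphere overlap with the TopDownCharacter shows a text prompt, enables input and opens a Gate, and leaving reverses all three.
; While the Gate is open, key 1 sets the HUD's left image and key 2 the right, using a shared flag to pick the branch.
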(event `Key|One`
  (params (Key :type "Key Structure"))
  (bind _hud (`/Game/TopDownBP/Blueprints/TopDownCharacter.hud` (`self.As Top Down Character`)))
  (:`Pressed`
    (set `self.flag` false)
    (`/Engine/EditorBlueprintResources/StandardMacros.Gate` true :!label _label
      (:`Exit`
        (if (`self.flag`)
          (`Image.SetBrushFromTexture` (`/Game/UI/MyHUD.Image_right` _hud) "/Game/UI/素材/-2.-2" false)
          (else
            (`Image.SetBrushFromTexture` (`/Game/UI/MyHUD.Image_left` _hud) "/Game/UI/素材/-1.-1" false)))))))

(event `Key|Two`
  (params (Key :type "Key Structure"))
  (:`Pressed`
    (set `self.flag` true)
    (goto _label)))

(event `self.Sphere.OnComponentBeginOverlap`
  (params (OverlappedComponent :type "PrimitiveComponent Object Reference") (OtherActor :type "Actor Object Reference") (OtherComp :type "PrimitiveComponent Object Reference") (OtherBodyIndex :type Integer) (bFromSweep :type Boolean) (SweepResult :type "HitResult Structure (by ref)"))
  (bind _astop_down_character (cast `/Game/TopDownBP/Blueprints/TopDownCharacter` OtherActor))
  (set `self.As Top Down Character` _astop_down_character)
  (`SceneComponent.SetVisibility` (`self.TextRender`) true false)
  (`self.EnableInput` (`GameplayStatics.GetPlayerController` 0))
  (goto _label :!via `Open`))

(event `self.Sphere.OnComponentEndOverlap`
  (params (OverlappedComponent :type "PrimitiveComponent Object Reference") (OtherActor :type "Actor Object Reference") (OtherComp :type "PrimitiveComponent Object Reference") (OtherBodyIndex :type Integer))
  (cast `/Game/TopDownBP/Blueprints/TopDownCharacter` OtherActor)
  (`SceneComponent.SetVisibility` (`self.TextRender`) false false)
  (`self.DisableInput` (`GameplayStatics.GetPlayerController` 0))
  (goto _label :!via `Close`))

(fn `UserConstructionScript`)
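; FinishTask_BP is an interaction point where the player turns in a mooncake gift box (月饼礼盒) to complete an order.
; Sphere overlap with the top-down character shows a text prompt, caches its HUD, enables input and opens a gate; leaving reverses this.
; Pressing E plays audio and, through the gate, SuccessFinished matches the held-item texture name and first board entry against HUD orders to clear them.
; Its Completed exit triggers StoryUMG hints via the game mode.
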(event `Key|E`
  (params (Key :type "Key Structure"))
  (:`Pressed`
    (`|ExecutionSequence`
      (:`then_0`
        (bind _returnvalue (`AddComponent|NODE_AddAudioComponent-2`))
        (`AudioComponent.Play` _returnvalue 0.0))
      (:`then_1`
        (`/Engine/EditorBlueprintResources/StandardMacros.Gate` true :!label _label
          (:`Exit`
            (`self.SuccessFinished`
              (:`Completed`
                (bind _astop_down_game_mode (cast `/Game/TopDownBP/Blueprints/TopDownGameMode` (`GameplayStatics.GetGameMode`)))
                (`/Game/UI/Story_UMG.CreateHints` (`/Game/TopDownBP/Blueprints/TopDownGameMode.StoryUMG` _astop_down_game_mode))))))))))

(event `self.Sphere.OnComponentBeginOverlap`
  (params (OverlappedComponent :type "PrimitiveComponent Object Reference") (OtherActor :type "Actor Object Reference") (OtherComp :type "PrimitiveComponent Object Reference") (OtherBodyIndex :type Integer) (bFromSweep :type Boolean) (SweepResult :type "HitResult Structure (by ref)"))
  (bind _astop_down_character (cast `/Game/TopDownBP/Blueprints/TopDownCharacter` OtherActor))
  (set `self.As Top Down Character` _astop_down_character)
  (set `self.hud` (`/Game/TopDownBP/Blueprints/TopDownCharacter.hud` _astop_down_character))
  (`SceneComponent.SetVisibility` (`self.TextRender`) true false)
  (`self.EnableInput` (`GameplayStatics.GetPlayerController` 0))
  (goto _label :!via `Open`))

(event `self.Sphere.OnComponentEndOverlap`
  (params (OverlappedComponent :type "PrimitiveComponent Object Reference") (OtherActor :type "Actor Object Reference") (OtherComp :type "PrimitiveComponent Object Reference") (OtherBodyIndex :type Integer))
  (cast `/Game/TopDownBP/Blueprints/TopDownCharacter` OtherActor)
  (`SceneComponent.SetVisibility` (`self.TextRender`) false false)
  (`self.DisableInput` (`GameplayStatics.GetPlayerController` 0))
  (goto _label :!via `Close`))

(fn `UserConstructionScript`)
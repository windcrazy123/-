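; Finishing board station where the player turns the items held in both hands into a raw white or green mooncake.
; Box overlap shows text prompts and opens a gate for the E key.
; Two checks read the HUD hand images' texture names, set the white/green flag from the right and append a combination code from the left to an array.
; It then swaps both HUD textures, leaving the raw mooncake on the left.
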(event `Key|E`
  (params (Key :type "Key Structure"))
  (bind _hud (`/Game/TopDownBP/Blueprints/TopDownCharacter.hud` (`self.As Top Down Character`)))
  (bind _image_right (`/Game/UI/MyHUD.Image_right` _hud))
  (bind _image_left (`/Game/UI/MyHUD.Image_left` _hud))
  (:`Pressed`
    (`/Engine/EditorBlueprintResources/StandardMacros.Gate` true :!label _label
      (:`Exit`
        (`self.right cannot` (`WidgetBlueprintLibrary.GetBrushResourceAsTexture2D` (`Image.Brush` _image_right))
          (:`else`
            (`self.left cannot` (`WidgetBlueprintLibrary.GetBrushResourceAsTexture2D` (`Image.Brush` _image_left))
              (:`else`
                (if (`self.is white`)
                  (`Image.SetBrushFromTexture` _image_left "/Game/UI/素材2/白月饼（生）.白月饼（生）" false)
                  (else
                    (`Image.SetBrushFromTexture` _image_left "/Game/UI/素材2/青月饼（生）.青月饼（生）" false)))
                (`Image.SetBrushFromTexture` _image_right "/Game/UI/素材/-2.-2" false)))))))))

(event `self.Box.OnComponentBeginOverlap`
  (params (OverlappedComponent :type "PrimitiveComponent Object Reference") (OtherActor :type "Actor Object Reference") (OtherComp :type "PrimitiveComponent Object Reference") (OtherBodyIndex :type Integer) (bFromSweep :type Boolean) (SweepResult :type "HitResult Structure (by ref)"))
  (bind _astop_down_character (cast `/Game/TopDownBP/Blueprints/TopDownCharacter` OtherActor))
  (set `self.As Top Down Character` _astop_down_character)
  (`SceneComponent.SetVisibility` (`self.TextRender`) true false)
  (`SceneComponent.SetVisibility` (`self.TextRender1`) true false)
  (`self.EnableInput` (`GameplayStatics.GetPlayerController` 0))
  (goto _label :!via `Open`))

(event `self.Box.OnComponentEndOverlap`
  (params (OverlappedComponent :type "PrimitiveComponent Object Reference") (OtherActor :type "Actor Object Reference") (OtherComp :type "PrimitiveComponent Object Reference") (OtherBodyIndex :type Integer))
  (cast `/Game/TopDownBP/Blueprints/TopDownCharacter` OtherActor)
  (`SceneComponent.SetVisibility` (`self.TextRender`) false false)
  (`SceneComponent.SetVisibility` (`self.TextRender1`) false false)
  (`self.DisableInput` (`GameplayStatics.GetPlayerController` 0))
  (goto _label :!via `Close`))

(fn `UserConstructionScript`)
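; Proximity interactable that changes the top-down character's left HUD image when E is pressed.
; Box overlap with the character shows or hides a text prompt, toggles input and opens or closes a gate on the key.
; The current texture's name serves as state: if numeric, it is converted to an integer, incremented and switched on to pick one of five hardcoded replacement textures.
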(event `Key|E`
  (params (Key :type "Key Structure"))
  (bind _image_left (`/Game/UI/MyHUD.Image_left` (`/Game/TopDownBP/Blueprints/TopDownCharacter.hud` (`self.As Top Down Character`))))
  (bind _returnvalue (`KismetSystemLibrary.GetObjectName` (`WidgetBlueprintLibrary.GetBrushResourceAsTexture2D` (`Image.Brush` _image_left))))
  (:`Pressed`
    (`/Engine/EditorBlueprintResources/StandardMacros.Gate` true :!label _label
      (:`Exit`
        (if (`KismetStringLibrary.IsNumeric` _returnvalue)
          (switch `int` (+ (`KismetStringLibrary.Conv_StringToInt` _returnvalue) 1)
            (:`0`
              (`Image.SetBrushFromTexture` _image_left "/Game/UI/素材2/2.2" false))
            (:`1`
              (`Image.SetBrushFromTexture` _image_left "/Game/UI/素材2/20.20" false))
            (:`2`
              (`Image.SetBrushFromTexture` _image_left "/Game/UI/素材2/1.1" false))
            (:`3`
              (`Image.SetBrushFromTexture` _image_left "/Game/UI/素材/-3.-3" false))
            (:`4`
              (`Image.SetBrushFromTexture` _image_left "/Game/UI/素材2/23.23" false))))))))

(event `self.Box.OnComponentBeginOverlap`
  (params (OverlappedComponent :type "PrimitiveComponent Object Reference") (OtherActor :type "Actor Object Reference") (OtherComp :type "PrimitiveComponent Object Reference") (OtherBodyIndex :type Integer) (bFromSweep :type Boolean) (SweepResult :type "HitResult Structure (by ref)"))
  (bind _astop_down_character (cast `/Game/TopDownBP/Blueprints/TopDownCharacter` OtherActor))
  (set `self.As Top Down Character` _astop_down_character)
  (`SceneComponent.SetVisibility` (`self.TextRender`) true false)
  (`self.EnableInput` (`GameplayStatics.GetPlayerController` 0))
  (goto _label :!via `Open`))

(event `self.Box.OnComponentEndOverlap`
  (params (OverlappedComponent :type "PrimitiveComponent Object Reference") (OtherActor :type "Actor Object Reference") (OtherComp :type "PrimitiveComponent Object Reference") (OtherBodyIndex :type Integer))
  (cast `/Game/TopDownBP/Blueprints/TopDownCharacter` OtherActor)
  (`SceneComponent.SetVisibility` (`self.TextRender`) false false)
  (`self.DisableInput` (`GameplayStatics.GetPlayerController` 0))
  (goto _label :!via `Close`))

(fn `UserConstructionScript`)
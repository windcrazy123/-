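; SubmitOrder is an order hand-in station: inside its box the player sees a text prompt and can press E to deliver held items.
; Overlap toggles input and a gate; E loops through HUD order images, matching brush texture names against both character hand images for two juices and a bowl of yuan.
; Matches hide the order, decrement its index, reset the hand image, increment Level2GameMode's SubmittedNum, call DengMi and activate audio.
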(event `self.ReceiveBeginPlay`)

(event `Key|E`
  (params (Key :type "Key Structure"))
  (bind _charactermessage (`/Game/TopDownBP/Blueprints/TopDownCharacter1.CharacterMessage` (`self.As Top Down Character 1`)))
  (bind _orderumg (`/Game/NewHUD.OrderUMG` (`self.As New HUD`)))
  (bind _charactermessage_2 (`/Game/TopDownBP/Blueprints/TopDownCharacter1.CharacterMessage` (`self.As Top Down Character 1`)))
  (bind _image_left2 (`/Game/UI/Level2UI/CharacterMessage.Image_left2` _charactermessage_2))
  (bind _image_right2 (`/Game/UI/Level2UI/CharacterMessage.Image_right2` _charactermessage_2))
  (bind _returnvalue (`KismetStringLibrary.Conv_ObjectToString` (`WidgetBlueprintLibrary.GetBrushResourceAsTexture2D` (`Image.Brush` (`/Game/UI/Level2UI/CharacterMessage.Image_right2` _charactermessage)))))
  (bind _returnvalue_2 (`KismetStringLibrary.Conv_ObjectToString` (`WidgetBlueprintLibrary.GetBrushResourceAsTexture2D` (`Image.Brush` (`/Game/UI/Level2UI/CharacterMessage.Image_left2` _charactermessage)))))
  (bind _returnvalue_3 (== _returnvalue_2 "kiwifruitJuice"))
  (bind _returnvalue_4 (== _returnvalue_2 "orangeJuice"))
  (bind _returnvalue_5 (== _returnvalue_2 "bowlOfYuan"))
  (:`Pressed`
    (`/Engine/EditorBlueprintResources/StandardMacros.Gate` true :!label _label
      (:`Exit`
        (bind _asnew_hud (cast `/Game/NewHUD` (`PlayerController.GetHUD` (`GameplayStatics.GetPlayerController` 0))))
        (bind _output_get (set `self.As New HUD` _asnew_hud))
        (for _array_element (`/Game/UI/Level2UI/OrderUMG.ImgArray` (`/Game/NewHUD.OrderUMG` _output_get))
          (bind _returnvalue_6 (`KismetStringLibrary.Conv_ObjectToString` (`WidgetBlueprintLibrary.GetBrushResourceAsTexture2D` (`Image.Brush` _array_element))))
          (bind _returnvalue_7 (and (== _returnvalue_6 "KiwifruitJuiceOrder") (or _returnvalue_3 (== _returnvalue "kiwifruitJuice"))))
          (bind _output_get_2 (set `self.NewVar_0` _returnvalue_7))
          (bind _returnvalue_8 (and (== _returnvalue_6 "OrangeJuiceOrder") (or _returnvalue_4 (== _returnvalue "orangeJuice"))))
          (bind _output_get_3 (set `self.NewVar_1` _returnvalue_8))
          (bind _returnvalue_9 (and (== _returnvalue_6 "YuanOrder") (or _returnvalue_5 (== _returnvalue "bowlOfYuan"))))
          (bind _output_get_4 (set `self.NewVar_2` _returnvalue_9))
          (bind _returnvalue_10 (or _returnvalue_7 _returnvalue_8 _returnvalue_9))
          (if _returnvalue_10
            (`Image.SetBrushFromSoftTexture` _array_element "/Game/UI/0NONE.0NONE" false)
            (`Widget.SetVisibility` _array_element "Hidden")
            (set `/Game/UI/Level2UI/OrderUMG.ImgArrayIndex` (- (`/Game/UI/Level2UI/OrderUMG.ImgArrayIndex` _orderumg) 1) _orderumg)
            (if _output_get_2
              (if _returnvalue_3
                (`Image.SetBrushFromSoftTexture` _image_left2 "/Game/UI/素材/-1.-1" false)
                (else
                  (`Image.SetBrushFromSoftTexture` _image_right2 "/Game/UI/素材/-2.-2" false)))
              (bind _aslevel_2game_mode (cast `/Game/TopDownBP/Blueprints/Level2GameMode` (`GameplayStatics.GetGameMode`) :!label _label_2))
              (set `/Game/TopDownBP/Blueprints/Level2GameMode.SubmittedNum` (+ (`/Game/TopDownBP/Blueprints/Level2GameMode.SubmittedNum` _aslevel_2game_mode) 1) _aslevel_2game_mode)
              (`/Game/TopDownBP/Blueprints/Level2GameMode.DengMi` _aslevel_2game_mode)
              (`ActorComponent.Activate` (`self.Audio`) false)
              (elif _output_get_3
                (if _returnvalue_4
                  (`Image.SetBrushFromSoftTexture` _image_left2 "/Game/UI/素材/-1.-1" false)
                  (goto _label_2)
                  (else
                    (`Image.SetBrushFromSoftTexture` _image_right2 "/Game/UI/素材/-2.-2" false)
                    (goto _label_2)))
                (elif _output_get_4
                  (if _returnvalue_5
                    (`Image.SetBrushFromSoftTexture` _image_left2 "/Game/UI/素材/-1.-1" false)
                    (goto _label_2)
                    (else
                      (`Image.SetBrushFromSoftTexture` _image_right2 "/Game/UI/素材/-2.-2" false)
                      (goto _label_2)))
                  (else
                    (`KismetSystemLibrary.PrintString` (`KismetStringLibrary.Conv_BoolToString` _returnvalue_10))))))))))))

(event `self.Box.OnComponentBeginOverlap`
  (params (OverlappedComponent :type "PrimitiveComponent Object Reference") (OtherActor :type "Actor Object Reference") (OtherComp :type "PrimitiveComponent Object Reference") (OtherBodyIndex :type Integer) (bFromSweep :type Boolean) (SweepResult :type "HitResult Structure (by ref)"))
  (bind _astop_down_character_1 (cast `/Game/TopDownBP/Blueprints/TopDownCharacter1` OtherActor))
  (set `self.As Top Down Character 1` _astop_down_character_1)
  (`SceneComponent.SetVisibility` (`self.TextRender`) true false)
  (`self.EnableInput` (`GameplayStatics.GetPlayerController` 0))
  (goto _label :!via `Open`))

(event `self.Box.OnComponentEndOverlap`
  (params (OverlappedComponent :type "PrimitiveComponent Object Reference") (OtherActor :type "Actor Object Reference") (OtherComp :type "PrimitiveComponent Object Reference") (OtherBodyIndex :type Integer))
  (cast `/Game/TopDownBP/Blueprints/TopDownCharacter1` OtherActor)
  (`SceneComponent.SetVisibility` (`self.TextRender`) false false)
  (`self.DisableInput` (`GameplayStatics.GetPlayerController` 0))
  (goto _label :!via `Close`))

(fn `UserConstructionScript`)
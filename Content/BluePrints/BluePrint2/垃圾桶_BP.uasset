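; Trash can interactable Blueprint that responds to the 1 and 2 keys while the TopDownCharacter1 is nearby.
; Sphere overlap stores the character, enables input and opens a gate; leaving disables input and closes it.
; Through that gate, key 1 changes the left image in the character's CharacterMessage widget, and key 2 changes the right image and prints a debug string.
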(event `Key|One`
  (params (Key :type "Key Structure"))
  (bind _charactermessage (`/Game/TopDownBP/Blueprints/TopDownCharacter1.CharacterMessage` (`self.As Top Down Character 1`)))
  (:`Pressed`
    (set `self.flag` false)
    (`/Engine/EditorBlueprintResources/StandardMacros.Gate` true :!label _label
      (:`Exit`
        (if (`self.flag`)
          (`KismetSystemLibrary.PrintString` "Hello")
          (`Image.SetBrushFromSoftTexture` (`/Game/UI/Level2UI/CharacterMessage.Image_right2` _charactermessage) "/Game/UI/素材/-2.-2" false)
          (else
            (`Image.SetBrushFromSoftTexture` (`/Game/UI/Level2UI/CharacterMessage.Image_left2` _charactermessage) "/Game/UI/素材/-1.-1" false)))))))

(event `Key|Two`
  (params (Key :type "Key Structure"))
  (:`Pressed`
    (set `self.flag` true)
    (goto _label)))

(event `self.Sphere.OnComponentBeginOverlap`
  (params (OverlappedComponent :type "PrimitiveComponent Object Reference") (OtherActor :type "Actor Object Reference") (OtherComp :type "PrimitiveComponent Object Reference") (OtherBodyIndex :type Integer) (bFromSweep :type Boolean) (SweepResult :type "HitResult Structure (by ref)"))
  (bind _astop_down_character_1 (cast `/Game/TopDownBP/Blueprints/TopDownCharacter1` OtherActor))
  (set `self.As Top Down Character 1` _astop_down_character_1)
  (`self.EnableInput` (`GameplayStatics.GetPlayerController` 0))
  (goto _label :!via `Open`))

(event `self.Sphere.OnComponentEndOverlap`
  (params (OverlappedComponent :type "PrimitiveComponent Object Reference") (OtherActor :type "Actor Object Reference") (OtherComp :type "PrimitiveComponent Object Reference") (OtherBodyIndex :type Integer))
  (cast `/Game/TopDownBP/Blueprints/TopDownCharacter1` OtherActor)
  (`self.DisableInput` (`GameplayStatics.GetPlayerController` 0))
  (goto _label :!via `Close`))

(fn `UserConstructionScript`)
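; Kitchen station actor where the player gathers ingredients, makes and cooks yuanxiao, takes bowls and juices fruit.
; Each station's overlap shows any prompt, enables input and opens a Gate that lets the E key act.
; Held items live only in the character widget's two hand images, identified by matching brush textures against HUD material arrays.
; The pot counts dumplings after a cook delay, a panel handles juicing, and a looping timer swaps kiwifruit and orange positions.
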(event `Key|E`
  (params (Key :type "Key Structure"))
  ;[1 1 1] Making Yuanxiao
  (:`Pressed`
    (`/Engine/EditorBlueprintResources/StandardMacros.Gate` true :!label _label
      (:`Exit`
        (`self.NewFunction_0` :!label _label_2)))))

(event `self.peanut.OnComponentBeginOverlap`
  (params (OverlappedComponent :type "PrimitiveComponent Object Reference") (OtherActor :type "Actor Object Reference") (OtherComp :type "PrimitiveComponent Object Reference") (OtherBodyIndex :type Integer) (bFromSweep :type Boolean) (SweepResult :type "HitResult Structure (by ref)"))
  ;[1 1 1] Making Yuanxiao
  (bind _astop_down_character_1 (cast `/Game/TopDownBP/Blueprints/TopDownCharacter1` OtherActor))
  (set `self.As Top Down Character 1` _astop_down_character_1)
  (`SceneComponent.SetVisibility` (`self.Peanut_text`) true false)
  (`self.EnableInput` (`GameplayStatics.GetPlayerController` 0))
  (set `self.materials_yuan` 1)
  (goto _label :!via `Open`))

(event `self.peanut.OnComponentEndOverlap`
  (params (OverlappedComponent :type "PrimitiveComponent Object Reference") (OtherActor :type "Actor Object Reference") (OtherComp :type "PrimitiveComponent Object Reference") (OtherBodyIndex :type Integer))
  ;[1 1 1] Making Yuanxiao
  (cast `/Game/TopDownBP/Blueprints/TopDownCharacter1` OtherActor)
  (`SceneComponent.SetVisibility` (`self.Peanut_text`) false false)
  (`self.DisableInput` (`GameplayStatics.GetPlayerController` 0))
  (goto _label :!via `Close`))

(event `Key|E`
  (params (Key :type "Key Structure"))
  ;[1 1 1] Making Yuanxiao
  (:`Pressed`
    (`/Engine/EditorBlueprintResources/StandardMacros.Gate` true
      (:`Exit`
        (goto _label_2)))))

(event `self.sesame.OnComponentBeginOverlap`
  (params (OverlappedComponent :type "PrimitiveComponent Object Reference") (OtherActor :type "Actor Object Reference") (OtherComp :type "PrimitiveComponent Object Reference") (OtherBodyIndex :type Integer) (bFromSweep :type Boolean) (SweepResult :type "HitResult Structure (by ref)"))
  ;[1 1 1] Making Yuanxiao
  (bind _astop_down_character_1 (cast `/Game/TopDownBP/Blueprints/TopDownCharacter1` OtherActor))
  (set `self.As Top Down Character 1` _astop_down_character_1)
  (`SceneComponent.SetVisibility` (`self.Sesame_text`) true false)
  (`self.EnableInput` (`GameplayStatics.GetPlayerController` 0))
  (set `self.materials_yuan` 0)
  (goto _label :!via `Open`))

(event `self.sesame.OnComponentEndOverlap`
  (params (OverlappedComponent :type "PrimitiveComponent Object Reference") (OtherActor :type "Actor Object Reference") (OtherComp :type "PrimitiveComponent Object Reference") (OtherBodyIndex :type Integer))
  ;[1 1 1] Making Yuanxiao
  (cast `/Game/TopDownBP/Blueprints/TopDownCharacter1` OtherActor)
  (`SceneComponent.SetVisibility` (`self.Sesame_text`) false false)
  (`self.DisableInput` (`GameplayStatics.GetPlayerController` 0))
  (goto _label :!via `Close`))

(event `Key|E`
  (params (Key :type "Key Structure"))
  (bind _charactermessage (`/Game/TopDownBP/Blueprints/TopDownCharacter1.CharacterMessage` (`self.As Top Down Character 1`)))
  (bind _materials_yuanxiao (`/Game/NewHUD.Materials_yuanxiao` (`self.As New HUD`)))
  (bind _charactermessage_2 (`/Game/TopDownBP/Blueprints/TopDownCharacter1.CharacterMessage` (`self.As Top Down Character 1`)))
  (bind _returnvalue (`KismetArrayLibrary.Array_Find` _materials_yuanxiao (`|ConvertAsset` (`WidgetBlueprintLibrary.GetBrushResourceAsTexture2D` (`Image.Brush` (`/Game/UI/Level2UI/CharacterMessage.Image_left2` _charactermessage))))))
  (bind _returnvalue_2 (`KismetArrayLibrary.Array_Find` _materials_yuanxiao (`|ConvertAsset` (`WidgetBlueprintLibrary.GetBrushResourceAsTexture2D` (`Image.Brush` (`/Game/UI/Level2UI/CharacterMessage.Image_right2` _charactermessage))))))
  ;[1 1 1] Making Yuanxiao
  (:`Pressed`
    (`/Engine/EditorBlueprintResources/StandardMacros.Gate` true :!label _label_3
      (:`Exit`
        (if (and (!= _returnvalue_2 -1) (!= _returnvalue -1) (!= _returnvalue_2 _returnvalue))
          (`Image.SetBrushFromSoftTexture` (`/Game/UI/Level2UI/CharacterMessage.Image_right2` _charactermessage_2) "/Game/UI/素材/-2.-2" false)
          (`Image.SetBrushFromSoftTexture` (`/Game/UI/Level2UI/CharacterMessage.Image_left2` _charactermessage_2) "/Game/UI/素材3/stuffing.stuffing" false))))))

(event `self.knife.OnComponentBeginOverlap`
  (params (OverlappedComponent :type "PrimitiveComponent Object Reference") (OtherActor :type "Actor Object Reference") (OtherComp :type "PrimitiveComponent Object Reference") (OtherBodyIndex :type Integer) (bFromSweep :type Boolean) (SweepResult :type "HitResult Structure (by ref)"))
  ;[1 1 1] Making Yuanxiao
  (bind _astop_down_character_1 (cast `/Game/TopDownBP/Blueprints/TopDownCharacter1` OtherActor))
  (set `self.As Top Down Character 1` _astop_down_character_1)
  (`SceneComponent.SetVisibility` (`self.knife_text`) true false)
  (`self.EnableInput` (`GameplayStatics.GetPlayerController` 0))
  (goto _label_3 :!via `Open`))

(event `self.knife.OnComponentEndOverlap`
  (params (OverlappedComponent :type "PrimitiveComponent Object Reference") (OtherActor :type "Actor Object Reference") (OtherComp :type "PrimitiveComponent Object Reference") (OtherBodyIndex :type Integer))
  ;[1 1 1] Making Yuanxiao
  (cast `/Game/TopDownBP/Blueprints/TopDownCharacter1` OtherActor)
  (`SceneComponent.SetVisibility` (`self.knife_text`) false false)
  (`self.DisableInput` (`GameplayStatics.GetPlayerController` 0))
  (goto _label_3 :!via `Close`))

(event `Key|E`
  (params (Key :type "Key Structure"))
  (bind _image_left2 (`/Game/UI/Level2UI/CharacterMessage.Image_left2` (`/Game/TopDownBP/Blueprints/TopDownCharacter1.CharacterMessage` (`self.As Top Down Character 1`))))
  ;[1 1 1] Making Yuanxiao
  (:`Pressed`
    (`/Engine/EditorBlueprintResources/StandardMacros.Gate` true :!label _label_4
      (:`Exit`
        (if (== (`KismetArrayLibrary.Array_Find` (`/Game/NewHUD.Materials` (`self.As New HUD`)) (`|ConvertAsset` (`WidgetBlueprintLibrary.GetBrushResourceAsTexture2D` (`Image.Brush` _image_left2)))) 0)
          (`Image.SetBrushFromSoftTexture` _image_left2 "/Game/UI/素材3/yuanxiao.yuanxiao" false))))))

(event `self.crust.OnComponentBeginOverlap`
  (params (OverlappedComponent :type "PrimitiveComponent Object Reference") (OtherActor :type "Actor Object Reference") (OtherComp :type "PrimitiveComponent Object Reference") (OtherBodyIndex :type Integer) (bFromSweep :type Boolean) (SweepResult :type "HitResult Structure (by ref)"))
  ;[1 1 1] Making Yuanxiao
  (bind _astop_down_character_1 (cast `/Game/TopDownBP/Blueprints/TopDownCharacter1` OtherActor))
  (set `self.As Top Down Character 1` _astop_down_character_1)
  (`SceneComponent.SetVisibility` (`self.crust_text`) true false)
  (`self.EnableInput` (`GameplayStatics.GetPlayerController` 0))
  (goto _label_4 :!via `Open`))

(event `self.crust.OnComponentEndOverlap`
  (params (OverlappedComponent :type "PrimitiveComponent Object Reference") (OtherActor :type "Actor Object Reference") (OtherComp :type "PrimitiveComponent Object Reference") (OtherBodyIndex :type Integer))
  ;[1 1 1] Making Yuanxiao
  (cast `/Game/TopDownBP/Blueprints/TopDownCharacter1` OtherActor)
  (`SceneComponent.SetVisibility` (`self.crust_text`) false false)
  (`self.DisableInput` (`GameplayStatics.GetPlayerController` 0))
  (goto _label_4 :!via `Close`))

(event `Key|E`
  (params (Key :type "Key Structure"))
  (bind _textrender (`self.TextRender`))
  (bind _charactermessage (`/Game/TopDownBP/Blueprints/TopDownCharacter1.CharacterMessage` (`self.As Top Down Character 1`)))
  (bind _materials (`/Game/NewHUD.Materials` (`self.As New HUD`)))
  (bind _charactermessage_2 (`/Game/TopDownBP/Blueprints/TopDownCharacter1.CharacterMessage` (`self.As Top Down Character 1`)))
  (bind _charactermessage_3 (`/Game/TopDownBP/Blueprints/TopDownCharacter1.CharacterMessage` (`self.As Top Down Character 1`)))
  (bind _charactermessage_4 (`/Game/TopDownBP/Blueprints/TopDownCharacter1.CharacterMessage` (`self.As Top Down Character 1`)))
  (bind _materials_2 (`/Game/NewHUD.Materials` (`self.As New HUD`)))
  (bind _returnvalue (== (`KismetArrayLibrary.Array_Find` _materials_2 (`|ConvertAsset` (`WidgetBlueprintLibrary.GetBrushResourceAsTexture2D` (`Image.Brush` (`/Game/UI/Level2UI/CharacterMessage.Image_left2` _charactermessage_2))))) 3))
  (bind _returnvalue_2 (== (`KismetArrayLibrary.Array_Find` _materials (`|ConvertAsset` (`WidgetBlueprintLibrary.GetBrushResourceAsTexture2D` (`Image.Brush` (`/Game/UI/Level2UI/CharacterMessage.Image_left2` _charactermessage))))) 2))
  ;[1 1 1] Cooking Yuanxiao
  (:`Pressed`
    (`/Engine/EditorBlueprintResources/StandardMacros.Gate` true :!label _label_5
      (:`Exit`
        (if (`self.IsHaveYuanInPot`)
          (if (or (== (`KismetArrayLibrary.Array_Find` _materials_2 (`|ConvertAsset` (`WidgetBlueprintLibrary.GetBrushResourceAsTexture2D` (`Image.Brush` (`/Game/UI/Level2UI/CharacterMessage.Image_right2` _charactermessage_2))))) 3) _returnvalue)
            (if (== _returnvalue true)
              (`Image.SetBrushFromSoftTexture` (`/Game/UI/Level2UI/CharacterMessage.Image_left2` _charactermessage_3) "/Game/UI/素材3/bowlOfYuan.bowlOfYuan" false)
              (else
                (`Image.SetBrushFromSoftTexture` (`/Game/UI/Level2UI/CharacterMessage.Image_right2` _charactermessage_3) "/Game/UI/素材3/bowlOfYuan.bowlOfYuan" false)))
            (bind _output_get (set `self.YuanNumInPot` (- (`self.YuanNumInPot`) 1)))
            (if (== _output_get 0)
              (set `self.IsHaveYuanInPot` false)
              (`SceneComponent.SetVisibility` _textrender false false)))
          (elif (or (== (`KismetArrayLibrary.Array_Find` _materials (`|ConvertAsset` (`WidgetBlueprintLibrary.GetBrushResourceAsTexture2D` (`Image.Brush` (`/Game/UI/Level2UI/CharacterMessage.Image_right2` _charactermessage))))) 2) _returnvalue_2)
            (if (== _returnvalue_2 true)
              (`Image.SetBrushFromSoftTexture` (`/Game/UI/Level2UI/CharacterMessage.Image_left2` _charactermessage_4) "/Game/UI/素材/-1.-1" false)
              (else
                (`Image.SetBrushFromSoftTexture` (`/Game/UI/Level2UI/CharacterMessage.Image_right2` _charactermessage_4) "/Game/UI/素材/-2.-2" false)))
            (`ActorComponent.Activate` (`self.Audio`) false)
            (`KismetSystemLibrary.Delay` 8.0)
            (set `self.IsHaveYuanInPot` true)
            (set `self.YuanNumInPot` (+ (`self.YuanNumInPot`) 1))
            (`SceneComponent.SetVisibility` _textrender true false)))))))

(event `self.pot.OnComponentBeginOverlap`
  (params (OverlappedComponent :type "PrimitiveComponent Object Reference") (OtherActor :type "Actor Object Reference") (OtherComp :type "PrimitiveComponent Object Reference") (OtherBodyIndex :type Integer) (bFromSweep :type Boolean) (SweepResult :type "HitResult Structure (by ref)"))
  ;[1 1 1] Cooking Yuanxiao
  (bind _astop_down_character_1 (cast `/Game/TopDownBP/Blueprints/TopDownCharacter1` OtherActor))
  (set `self.As Top Down Character 1` _astop_down_character_1)
  (`SceneComponent.SetVisibility` (`self.pot_text`) true false)
  (`self.EnableInput` (`GameplayStatics.GetPlayerController` 0))
  (goto _label_5 :!via `Open`))

(event `self.pot.OnComponentEndOverlap`
  (params (OverlappedComponent :type "PrimitiveComponent Object Reference") (OtherActor :type "Actor Object Reference") (OtherComp :type "PrimitiveComponent Object Reference") (OtherBodyIndex :type Integer))
  ;[1 1 1] Cooking Yuanxiao
  (cast `/Game/TopDownBP/Blueprints/TopDownCharacter1` OtherActor)
  (`SceneComponent.SetVisibility` (`self.pot_text`) false false)
  (`self.DisableInput` (`GameplayStatics.GetPlayerController` 0))
  (goto _label_5 :!via `Close`))

(event `Key|E`
  (params (Key :type "Key Structure"))
  (bind _as_new_hud (`self.As New HUD`))
  (bind _charactermessage (`/Game/TopDownBP/Blueprints/TopDownCharacter1.CharacterMessage` (`self.As Top Down Character 1`)))
  (bind _materials (`/Game/NewHUD.Materials` _as_new_hud))
  (bind _materials_yuanxiao (`/Game/NewHUD.Materials_yuanxiao` _as_new_hud))
  (bind _charactermessage_2 (`/Game/TopDownBP/Blueprints/TopDownCharacter1.CharacterMessage` (`self.As Top Down Character 1`)))
  (bind _output (`|ConvertAsset` (`WidgetBlueprintLibrary.GetBrushResourceAsTexture2D` (`Image.Brush` (`/Game/UI/Level2UI/CharacterMessage.Image_right2` _charactermessage)))))
  (bind _output_2 (`|ConvertAsset` (`WidgetBlueprintLibrary.GetBrushResourceAsTexture2D` (`Image.Brush` (`/Game/UI/Level2UI/CharacterMessage.Image_left2` _charactermessage)))))
  (bind _returnvalue (== (`KismetArrayLibrary.Array_Find` _materials_yuanxiao _output_2) -1))
  (bind _returnvalue_2 (== (`KismetArrayLibrary.Array_Find` _materials _output_2) -1))
  ;[1 1 1] Cooking Yuanxiao
  (:`Pressed`
    (`/Engine/EditorBlueprintResources/StandardMacros.Gate` true :!label _label_6
      (:`Exit`
        (if (and (or (== (`KismetArrayLibrary.Array_Find` _materials _output) -1) _returnvalue_2) (or (== (`KismetArrayLibrary.Array_Find` _materials_yuanxiao _output) -1) _returnvalue))
          (if (and (== _returnvalue_2 true) (== _returnvalue true))
            (`Image.SetBrushFromSoftTexture` (`/Game/UI/Level2UI/CharacterMessage.Image_left2` _charactermessage_2) "/Game/UI/素材3/bowl.bowl" false)
            (else
              (`Image.SetBrushFromSoftTexture` (`/Game/UI/Level2UI/CharacterMessage.Image_right2` _charactermessage_2) "/Game/UI/素材3/bowl.bowl" false))))))))

(event `self.bowl.OnComponentBeginOverlap`
  (params (OverlappedComponent :type "PrimitiveComponent Object Reference") (OtherActor :type "Actor Object Reference") (OtherComp :type "PrimitiveComponent Object Reference") (OtherBodyIndex :type Integer) (bFromSweep :type Boolean) (SweepResult :type "HitResult Structure (by ref)"))
  ;[1 1 1] Cooking Yuanxiao
  (bind _astop_down_character_1 (cast `/Game/TopDownBP/Blueprints/TopDownCharacter1` OtherActor))
  (set `self.As Top Down Character 1` _astop_down_character_1)
  (`SceneComponent.SetVisibility` (`self.bowl_text`) true false)
  (`self.EnableInput` (`GameplayStatics.GetPlayerController` 0))
  (goto _label_6 :!via `Open`))

(event `self.bowl.OnComponentEndOverlap`
  (params (OverlappedComponent :type "PrimitiveComponent Object Reference") (OtherActor :type "Actor Object Reference") (OtherComp :type "PrimitiveComponent Object Reference") (OtherBodyIndex :type Integer))
  ;[1 1 1] Cooking Yuanxiao
  (cast `/Game/TopDownBP/Blueprints/TopDownCharacter1` OtherActor)
  (`SceneComponent.SetVisibility` (`self.bowl_text`) false false)
  (`self.DisableInput` (`GameplayStatics.GetPlayerController` 0))
  (goto _label_6 :!via `Close`))

(event `Key|E`
  (params (Key :type "Key Structure"))
  (bind _as_new_hud (`self.As New HUD`))
  (bind _charactermessage (`/Game/TopDownBP/Blueprints/TopDownCharacter1.CharacterMessage` (`self.As Top Down Character 1`)))
  (bind _materials (`/Game/NewHUD.Materials` _as_new_hud))
  (bind _materials_yuanxiao (`/Game/NewHUD.Materials_yuanxiao` _as_new_hud))
  (bind _charactermessage_2 (`/Game/TopDownBP/Blueprints/TopDownCharacter1.CharacterMessage` (`self.As Top Down Character 1`)))
  (bind _output (`|ConvertAsset` (`WidgetBlueprintLibrary.GetBrushResourceAsTexture2D` (`Image.Brush` (`/Game/UI/Level2UI/CharacterMessage.Image_right2` _charactermessage)))))
  (bind _output_2 (`|ConvertAsset` (`WidgetBlueprintLibrary.GetBrushResourceAsTexture2D` (`Image.Brush` (`/Game/UI/Level2UI/CharacterMessage.Image_left2` _charactermessage)))))
  (bind _returnvalue (== (`KismetArrayLibrary.Array_Find` _materials_yuanxiao _output_2) -1))
  (bind _returnvalue_2 (== (`KismetArrayLibrary.Array_Find` _materials _output_2) -1))
  ;[1 1 1] Dress Fruit
  (:`Pressed`
    (`/Engine/EditorBlueprintResources/StandardMacros.Gate` true :!label _label_7
      (:`Exit`
        (if (and (or (== (`KismetArrayLibrary.Array_Find` _materials _output) -1) _returnvalue_2) (or (== (`KismetArrayLibrary.Array_Find` _materials_yuanxiao _output) -1) _returnvalue))
          (if (and (== _returnvalue_2 true) (== _returnvalue true))
            (`Image.SetBrushFromSoftTexture` (`/Game/UI/Level2UI/CharacterMessage.Image_left2` _charactermessage_2) "/Game/UI/素材3/kiwifruit.kiwifruit" false)
            (else
              (`Image.SetBrushFromSoftTexture` (`/Game/UI/Level2UI/CharacterMessage.Image_right2` _charactermessage_2) "/Game/UI/素材3/kiwifruit.kiwifruit" false))))))))

(event `self.kiwifruit.OnComponentBeginOverlap`
  (params (OverlappedComponent :type "PrimitiveComponent Object Reference") (OtherActor :type "Actor Object Reference") (OtherComp :type "PrimitiveComponent Object Reference") (OtherBodyIndex :type Integer) (bFromSweep :type Boolean) (SweepResult :type "HitResult Structure (by ref)"))
  ;[1 1 1] Dress Fruit
  (bind _astop_down_character_1 (cast `/Game/TopDownBP/Blueprints/TopDownCharacter1` OtherActor))
  (set `self.As Top Down Character 1` _astop_down_character_1)
  (`self.EnableInput` (`GameplayStatics.GetPlayerController` 0))
  (goto _label_7 :!via `Open`))

(event `self.kiwifruit.OnComponentEndOverlap`
  (params (OverlappedComponent :type "PrimitiveComponent Object Reference") (OtherActor :type "Actor Object Reference") (OtherComp :type "PrimitiveComponent Object Reference") (OtherBodyIndex :type Integer))
  ;[1 1 1] Dress Fruit
  (cast `/Game/TopDownBP/Blueprints/TopDownCharacter1` OtherActor)
  (`self.DisableInput` (`GameplayStatics.GetPlayerController` 0))
  (goto _label_7 :!via `Close`))

(event `Key|E`
  (params (Key :type "Key Structure"))
  (bind _as_new_hud (`self.As New HUD`))
  (bind _charactermessage (`/Game/TopDownBP/Blueprints/TopDownCharacter1.CharacterMessage` (`self.As Top Down Character 1`)))
  (bind _materials (`/Game/NewHUD.Materials` _as_new_hud))
  (bind _materials_yuanxiao (`/Game/NewHUD.Materials_yuanxiao` _as_new_hud))
  (bind _charactermessage_2 (`/Game/TopDownBP/Blueprints/TopDownCharacter1.CharacterMessage` (`self.As Top Down Character 1`)))
  (bind _output (`|ConvertAsset` (`WidgetBlueprintLibrary.GetBrushResourceAsTexture2D` (`Image.Brush` (`/Game/UI/Level2UI/CharacterMessage.Image_right2` _charactermessage)))))
  (bind _output_2 (`|ConvertAsset` (`WidgetBlueprintLibrary.GetBrushResourceAsTexture2D` (`Image.Brush` (`/Game/UI/Level2UI/CharacterMessage.Image_left2` _charactermessage)))))
  (bind _returnvalue (== (`KismetArrayLibrary.Array_Find` _materials_yuanxiao _output_2) -1))
  (bind _returnvalue_2 (== (`KismetArrayLibrary.Array_Find` _materials _output_2) -1))
  ;[1 1 1] Dress Fruit
  (:`Pressed`
    (`/Engine/EditorBlueprintResources/StandardMacros.Gate` true :!label _label_8
      (:`Exit`
        (if (and (or (== (`KismetArrayLibrary.Array_Find` _materials _output) -1) _returnvalue_2) (or (== (`KismetArrayLibrary.Array_Find` _materials_yuanxiao _output) -1) _returnvalue))
          (if (and (== _returnvalue_2 true) (== _returnvalue true))
            (`Image.SetBrushFromSoftTexture` (`/Game/UI/Level2UI/CharacterMessage.Image_left2` _charactermessage_2) "/Game/UI/素材3/orange.orange" false)
            (else
              (`Image.SetBrushFromSoftTexture` (`/Game/UI/Level2UI/CharacterMessage.Image_right2` _charactermessage_2) "/Game/UI/素材3/orange.orange" false))))))))

(event `self.orange.OnComponentBeginOverlap`
  (params (OverlappedComponent :type "PrimitiveComponent Object Reference") (OtherActor :type "Actor Object Reference") (OtherComp :type "PrimitiveComponent Object Reference") (OtherBodyIndex :type Integer) (bFromSweep :type Boolean) (SweepResult :type "HitResult Structure (by ref)"))
  ;[1 1 1] Dress Fruit
  (bind _astop_down_character_1 (cast `/Game/TopDownBP/Blueprints/TopDownCharacter1` OtherActor))
  (set `self.As Top Down Character 1` _astop_down_character_1)
  (`self.EnableInput` (`GameplayStatics.GetPlayerController` 0))
  (goto _label_8 :!via `Open`))

(event `self.orange.OnComponentEndOverlap`
  (params (OverlappedComponent :type "PrimitiveComponent Object Reference") (OtherActor :type "Actor Object Reference") (OtherComp :type "PrimitiveComponent Object Reference") (OtherBodyIndex :type Integer))
  ;[1 1 1] Dress Fruit
  (cast `/Game/TopDownBP/Blueprints/TopDownCharacter1` OtherActor)
  (`self.DisableInput` (`GameplayStatics.GetPlayerController` 0))
  (goto _label_8 :!via `Close`))

(event `Key|E`
  (params (Key :type "Key Structure"))
  (bind _charactermessage (`/Game/TopDownBP/Blueprints/TopDownCharacter1.CharacterMessage` (`self.As Top Down Character 1`)))
  (bind _materials (`/Game/NewHUD.Materials` (`self.As New HUD`)))
  (bind _returnvalue (`KismetArrayLibrary.Array_Find` _materials (`|ConvertAsset` (`WidgetBlueprintLibrary.GetBrushResourceAsTexture2D` (`Image.Brush` (`/Game/UI/Level2UI/CharacterMessage.Image_right2` _charactermessage))))))
  (bind _returnvalue_2 (`KismetArrayLibrary.Array_Find` _materials (`|ConvertAsset` (`WidgetBlueprintLibrary.GetBrushResourceAsTexture2D` (`Image.Brush` (`/Game/UI/Level2UI/CharacterMessage.Image_left2` _charactermessage))))))
  (bind _returnvalue_3 (== _returnvalue_2 5))
  (bind _returnvalue_4 (== _returnvalue 6))
  (bind _returnvalue_5 (== _returnvalue_2 6))
  ;[1 1 1] Dress Fruit
  (:`Pressed`
    (`/Engine/EditorBlueprintResources/StandardMacros.Gate` true :!label _label_9
      (:`Exit`
        (if (or (== _returnvalue 5) _returnvalue_4 _returnvalue_3 _returnvalue_5)
          (`self.DisposalFruit` (or _returnvalue_3 _returnvalue_5) _returnvalue_4 _returnvalue_5)
          (`self.Display Panel`)
          (add `UserWidget.OnVisibilityChanged` (`self.JuicerPanel`) (delegate `自定义事件_1`)))))))

(event `self.Juicer.OnComponentBeginOverlap`
  (params (OverlappedComponent :type "PrimitiveComponent Object Reference") (OtherActor :type "Actor Object Reference") (OtherComp :type "PrimitiveComponent Object Reference") (OtherBodyIndex :type Integer) (bFromSweep :type Boolean) (SweepResult :type "HitResult Structure (by ref)"))
  ;[1 1 1] Dress Fruit
  (bind _astop_down_character_1 (cast `/Game/TopDownBP/Blueprints/TopDownCharacter1` OtherActor))
  (set `self.As Top Down Character 1` _astop_down_character_1)
  (`SceneComponent.SetVisibility` (`self.juicer_text`) true false)
  (`self.InitJuicerPanel`)
  (`self.EnableInput` (`GameplayStatics.GetPlayerController` 0))
  (goto _label_9 :!via `Open`))

(event `self.Juicer.OnComponentEndOverlap`
  (params (OverlappedComponent :type "PrimitiveComponent Object Reference") (OtherActor :type "Actor Object Reference") (OtherComp :type "PrimitiveComponent Object Reference") (OtherBodyIndex :type Integer))
  ;[1 1 1] Dress Fruit
  (cast `/Game/TopDownBP/Blueprints/TopDownCharacter1` OtherActor)
  (`SceneComponent.SetVisibility` (`self.juicer_text`) false false)
  (`self.DisableInput` (`GameplayStatics.GetPlayerController` 0))
  (goto _label_9 :!via `Close`))

(event `自定义事件_1`
  (params (InVisibility :type "ESlateVisibility Enum" :default "Visible"))
  (bind _juicerpanel (`self.JuicerPanel`))
  (bind _charactermessage (`/Game/TopDownBP/Blueprints/TopDownCharacter1.CharacterMessage` (`self.As Top Down Character 1`)))
  (bind _image_left2 (`/Game/UI/Level2UI/CharacterMessage.Image_left2` _charactermessage))
  (bind _image_right2 (`/Game/UI/Level2UI/CharacterMessage.Image_right2` _charactermessage))
  ;[1 1 1] Dress Fruit
  (if (`Widget.IsVisible` _juicerpanel)
    _
    (elif (`/Game/UI/Level2UI/JuicerPanel.IsCanGetJuice` _juicerpanel)
      (if (`self.Is Left Have`)
        (if (`self.Is Left Have Orange`)
          (`Image.SetBrushFromSoftTexture` _image_left2 "/Game/UI/素材3/orangeJuice.orangeJuice" false)
          (else
            (`Image.SetBrushFromSoftTexture` _image_left2 "/Game/UI/素材3/kiwifruitJuice.kiwifruitJuice" false)))
        (elif (`self.Is Right Have Orange`)
          (`Image.SetBrushFromSoftTexture` _image_right2 "/Game/UI/素材3/orangeJuice.orangeJuice" false)
          (else
            (`Image.SetBrushFromSoftTexture` _image_right2 "/Game/UI/素材3/kiwifruitJuice.kiwifruitJuice" false))))
      (`ActorComponent.Activate` (`self.Audio1`) false))))

(event `self.ReceiveBeginPlay`
  ;[1 1 1] 初始化并设置ExchangeTimer
  (set `self.As New HUD` (cast `/Game/NewHUD` (`PlayerController.GetHUD` (`GameplayStatics.GetPlayerController` 0)) :!pure true))
  (`KismetSystemLibrary.K2_SetTimerDelegate` (delegate `Exchange`) 3.0 true))

(event `Exchange`
  ;[1 1 1] 初始化并设置ExchangeTimer
  (`self.ExchangeLocation` (`self.kiwifruit`) (`self.orange`)))

(fn `Display Panel`
  (bind _juicerpanel (`self.JuicerPanel`))
  (`WidgetBlueprintLibrary.SetInputMode_UIOnlyEx` (`GameplayStatics.GetPlayerController` 0) _juicerpanel)
  (`Widget.SetVisibility` _juicerpanel "Visible")
  (`UserWidget.PlayAnimationForward` _juicerpanel (`/Game/UI/Level2UI/JuicerPanel.NewAnimation` _juicerpanel) 1.0 false)
  (return))

(fn `DisposalFruit`
  (params (IsLeftHave :type Boolean) (IsRightHaveOrange :type Boolean) (IsLeftHaveOrange :type Boolean))
  (bind _charactermessage (`/Game/TopDownBP/Blueprints/TopDownCharacter1.CharacterMessage` (`self.As Top Down Character 1`)))
  (bind _output_get (set `self.Is Left Have` IsLeftHave))
  (set `self.Is Right Have Orange` IsRightHaveOrange)
  (set `self.Is Left Have Orange` IsLeftHaveOrange)
  (if _output_get
    (`Image.SetBrushFromSoftTexture` (`/Game/UI/Level2UI/CharacterMessage.Image_left2` _charactermessage) "/Game/UI/素材/-1.-1" false)
    (else
      (`Image.SetBrushFromSoftTexture` (`/Game/UI/Level2UI/CharacterMessage.Image_right2` _charactermessage) "/Game/UI/素材/-2.-2" false))))

(fn `ExchangeLocation`
  (params (ObjectA :type "SceneComponent Object Reference") (ObjectB :type "SceneComponent Object Reference"))
  (locals (NewLocalVar_1 :type "Vector Structure" :default (0.0 0.0 0.0)))
  (bind _output_get (set `local.NewLocalVar_1` (- (`SceneComponent.K2_GetComponentLocation` ObjectA) (`SceneComponent.K2_GetComponentLocation` ObjectB))))
  (`SceneComponent.K2_AddWorldOffset` ObjectB _output_get false false)
  (`SceneComponent.K2_AddWorldOffset` ObjectA (- (0.0 0.0 0.0) _output_get) false false))

(fn `InitJuicerPanel`
  (`/Engine/EditorBlueprintResources/StandardMacros.IsValid` (`self.JuicerPanel`)
    (:`Is Not Valid`
      (bind _returnvalue (`|CreateWidget` "/Game/UI/Level2UI/JuicerPanel.JuicerPanel_C"))
      (bind _output_get (set `self.JuicerPanel` _returnvalue))
      (`UserWidget.AddToViewport` _output_get 0)
      (`Widget.SetVisibility` _output_get "Hidden")
      (return))))

(fn `NewFunction_0`
  (locals (NewLocalVar_0 :type "/Game/NewHUD Object Reference"))
  (bind _charactermessage (`/Game/TopDownBP/Blueprints/TopDownCharacter1.CharacterMessage` (`self.As Top Down Character 1`)))
  (bind _output (`|GetArrayItem` (`/Game/NewHUD.Materials_yuanxiao` (`self.As New HUD`)) (`KismetMathLibrary.Conv_ByteToInt` (`self.materials_yuan`))))
  (bind _image_left2 (`/Game/UI/Level2UI/CharacterMessage.Image_left2` _charactermessage))
  (bind _image_right2 (`/Game/UI/Level2UI/CharacterMessage.Image_right2` _charactermessage))
  (if (`KismetStringLibrary.EqualEqual_StrStr` (`KismetSystemLibrary.GetObjectName` (`WidgetBlueprintLibrary.GetBrushResourceAsTexture2D` (`Image.Brush` _image_left2))) "-1")
    (`Image.SetBrushFromSoftTexture` _image_left2 _output false)
    (elif (`KismetStringLibrary.EqualEqual_StrStr` (`KismetSystemLibrary.GetObjectName` (`WidgetBlueprintLibrary.GetBrushResourceAsTexture2D` (`Image.Brush` _image_right2))) "-2")
      (`Image.SetBrushFromSoftTexture` _image_right2 _output false))))

(fn `UserConstructionScript`)